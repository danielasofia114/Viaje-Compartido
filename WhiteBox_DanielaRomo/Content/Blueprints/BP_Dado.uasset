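; BP_Dado is a dice duel in which the player rolls against an opponent, with Spanish on-screen messages.
; Tick polls the Boton flag and, when it is true, generates two random rolls from 1 to 5, one per side.
; It prints both results, compares them to announce a tie, win or loss through PrintString, then clears the flag so each trigger plays one round.
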(event `self.ReceiveTick`
  (params (DeltaSeconds :type "Float (single-precision)"))
  (if (`self.Boton`)
    (`KismetSystemLibrary.PrintString` "Tira los dados")
    (bind _result (`/Engine/EditorBlueprintResources/StandardMacros.IncrementInt` (`KismetMathLibrary.RandomInteger` 5))
      (:`  `
        (`KismetSystemLibrary.PrintString` (`KismetStringLibrary.Concat_StrStr` "Sacaste " (`KismetStringLibrary.Conv_IntToString` _result)))
        (bind _result_2 (`/Engine/EditorBlueprintResources/StandardMacros.IncrementInt` (`KismetMathLibrary.RandomInteger` 5))
          (:`  `
            (`KismetSystemLibrary.PrintString` (`KismetStringLibrary.Concat_StrStr` "Tu oponente sacó " (`KismetStringLibrary.Conv_IntToString` _result_2)))
            (if (== _result _result_2)
              (`KismetSystemLibrary.PrintString` "Hubo un empate")
              (elif (> _result _result_2)
                (`KismetSystemLibrary.PrintString` "¡Felicitaciones, ganaste!")
                (else
                  (`KismetSystemLibrary.PrintString` "Lo sentimos, perdiste"))))
            (set `self.Boton` false)))))))

(fn `UserConstructionScript`)