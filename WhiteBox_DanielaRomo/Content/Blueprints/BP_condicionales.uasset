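; BP_condicionales is a Blueprint exercise in nested conditionals that simulates a venue entry check by age and gender.
; On Tick, when the Boton flag is set, it branches on whether Edad marks an adult, then on Hombre for adults.
; Each outcome prints a Spanish message for cover charge, free drink or minor, then Boton resets so the check runs once per press.
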(event `self.ReceiveTick`
  (params (DeltaSeconds :type "Float (single-precision)"))
  (if (`self.Boton`)
    (if (> (`self.Edad`) 17)
      (`KismetSystemLibrary.PrintString` "Mayor de edad")
      (if (`self.Hombre`)
        (`KismetSystemLibrary.PrintString` "Cover 50.000")
        (else
          (`KismetSystemLibrary.PrintString` "Pola gratis")))
      (else
        (`KismetSystemLibrary.PrintString` "Menor de edad")))
    (set `self.Boton` false)))

(fn `UserConstructionScript`)